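; Game mode for a checkpoint time-trial racing game that spawns and possesses the garage-selected car and runs the race.
; Track info and difficulty set a countdown, which checkpoints hit in order extend, while a second timer tracks total time.
; Running out of time shows the loss screen.
; The final checkpoint pays a difficulty-based reward, saves per-map clears, unlocks cars by money and clears, and shows the win screen.
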(event Custom|TillRaceComplete
  ;[0.15 0.15 0.15 0.5] Time taken to complete the race calculation
  (Math|Float|IncrementFloat (Variables|Default|GetTOTAL_TIME%20)))

(event Custom|OnRaceTimerTick
  (if (Utilities|Enum|Equal(Enum) (Variables|Default|GetRaceState) "NewEnumerator1")
    (bind _returnvalue (Utilities|Time|SetTimerbyEvent (delegate Custom|OnRaceTimerTick) 1.0 true))
    (Variables|Default|SetRaceTimerHandle _returnvalue)
    (bind _output_get (Variables|Default|SetRemainingTime (- (Variables|Default|GetRemainingTime) 1.0)))
    (if (<= _output_get 0.0)
      (Variables|Default|SetRaceState "NewEnumerator2")
      (Utilities|Time|ClearandInvalidateTimerbyHandle (Variables|Default|GetRaceTimerHandle))
      (bind _returnvalue_2 (Game|GetCurrentLevelName true))
      (if (not (Utilities|Enum|Equal(Enum) _returnvalue_2 "Showroom_Level"))
        (bind _asbp_player_controller (Utilities|Casting|CastToBP_PlayerController (Game|GetPlayerController 0)))
        (Viewport|RemoveAllWidgets)
        (Default|SwitchtoCinematicCameralost _asbp_player_controller)
        (Default|ShowRewardsUILost _asbp_player_controller (Variables|/Game/SHOWROOM/MAIN/BP_PlayerCustomSave.BP_PlayerCustomSave_C|GetPlayerCurrency (Class|EMSFunctionLibrary|GetCustomSave "/Game/SHOWROOM/MAIN/BP_PlayerCustomSave.BP_PlayerCustomSave_C")) (Variables|Default|GetTOTAL_TIME%20))))))

(event EventBeginPlay
  (Utilities|FlowControl|Sequence
    (:then_0
      ;[0.15 0.15 0.15 0.5] THIS IS USED TO SPAWN THE CAR SELECTEDD IN GARAGE AT RUNTIME
      (bind _asbp_game_instance (Utilities|Casting|CastToBP_GameInstance (Game|GetGameInstance)))
      (Utilities|IsValid _asbp_game_instance
        (:Is%20Valid
          (bind _returnvalue (Game|SpawnActorfromClass (Variables|/Game/SHOWROOM/MAIN/BP_GameInstance.BP_GameInstance_C|GetCar%20Class _asbp_game_instance) (Transformation|GetActorTransform (Class|GameModeBase|FindPlayerStart (Game|GetPlayerController 0) "Player Start")) "Undefined" "MultiplyWithRoot" 0 0))
          (Pawn|Possess (Game|GetPlayerController 0) _returnvalue)
          (Utilities|FlowControl|Delay 1.0)
          (bind _returnvalue_2 (UserInterface|CreateWidget "/Game/CARS/UI_OF_ALL/WB_Cars_Racing_uI.WB_Cars_Racing_uI_C"))
          (UserInterface|Viewport|AddtoViewport _returnvalue_2 0))
        (:Is%20Not%20Valid
          (Development|PrintString "NO CAR SELECTED"))))
    (:then_1
      (bind _returnvalue_3 (Game|GetCurrentLevelName true))
      (Variables|Default|SetCurrentMapNamePlayed _returnvalue_3)
      (if (not (or (or (Utilities|Enum|Equal(Enum) _returnvalue_3 "MAINMENU_") (Utilities|Enum|Equal(Enum) _returnvalue_3 "Showroom_Level")) (or false (Utilities|Enum|Equal(Enum) _returnvalue_3 "Garage_Level"))))
        (bind _outactors (Actor|GetAllActorsOfClass "/Game/GAMERULES/BP_TrackInfo.BP_TrackInfo_C"))
        (bind _output_get (Variables|Default|SetTrackInfoRef (Utilities|Array|Get(acopy) _outactors)))
        (bind _output_get_2 (Variables|Default|SetTrackData (Variables|/Game/GAMERULES/BP_TrackInfo.BP_TrackInfo_C|GetTrackData _output_get)))
        (Variables|Default|SetSelected%20Difficulty%20Levelhggf (Variables|/Game/SHOWROOM/MAIN/BP_GameInstance.BP_GameInstance_C|GetSelectedDifficultyLevelhggf _asbp_game_instance))
        (switch Utilities|FlowControl|Switch|SwitchonE_Difficulty (Variables|/Game/SHOWROOM/MAIN/BP_GameInstance.BP_GameInstance_C|GetSelectedDifficultyLevelhggf _asbp_game_instance)
          (:NewEnumerator0
            (if (Utilities|Enum|Equal(Enum) (Variables|/Game/SHOWROOM/MAIN/BP_GameInstance.BP_GameInstance_C|GetSelectedDifficultyLevelhggf _asbp_game_instance) "NewEnumerator0")
              (Variables|Default|SetRemainingTime (.EasyInitialTime (Utilities|Struct|BreakS_TrackData _output_get_2)))
              (Variables|Default|SetCheckpointTimeBonus (.EasyCheckpointBonus (Utilities|Struct|BreakS_TrackData _output_get_2)))
              (Variables|Default|SetRaceState "NewEnumerator1" :!label _label)
              (bind _returnvalue_4 (Utilities|Time|SetTimerbyEvent (delegate Custom|OnRaceTimerTick) 1.0 true))
              (Variables|Default|SetRaceTimerHandle _returnvalue_4)
              (bind _output_get_3 (Variables|Default|SetRemainingTime (- (Variables|Default|GetRemainingTime) 1.0)))
              (if (<= _output_get_3 0.0)
                (Variables|Default|SetRaceState "NewEnumerator2")
                (Utilities|Time|ClearandInvalidateTimerbyHandle (Variables|Default|GetRaceTimerHandle))
                (bind _returnvalue_5 (Game|GetCurrentLevelName true))
                (if (not (Utilities|Enum|Equal(Enum) _returnvalue_5 "Showroom_Level"))
                  (bind _asbp_player_controller (Utilities|Casting|CastToBP_PlayerController (Game|GetPlayerController 0)))
                  (Viewport|RemoveAllWidgets)
                  (Default|SwitchtoCinematicCameralost _asbp_player_controller)
                  (Default|ShowRewardsUILost _asbp_player_controller (Variables|/Game/SHOWROOM/MAIN/BP_PlayerCustomSave.BP_PlayerCustomSave_C|GetPlayerCurrency (Class|EMSFunctionLibrary|GetCustomSave "/Game/SHOWROOM/MAIN/BP_PlayerCustomSave.BP_PlayerCustomSave_C")) (Variables|Default|GetTOTAL_TIME%20))))))
          (:NewEnumerator1
            (if (Utilities|Enum|Equal(Enum) (Variables|/Game/SHOWROOM/MAIN/BP_GameInstance.BP_GameInstance_C|GetSelectedDifficultyLevelhggf _asbp_game_instance) "NewEnumerator1")
              (Variables|Default|SetRemainingTime (.MediumInitialTime (Utilities|Struct|BreakS_TrackData _output_get_2)))
              (Variables|Default|SetCheckpointTimeBonus (.MediumCheckpointBonus (Utilities|Struct|BreakS_TrackData _output_get_2)))
              (goto _label)))
          (:NewEnumerator2
            (if (Utilities|Enum|Equal(Enum) (Variables|/Game/SHOWROOM/MAIN/BP_GameInstance.BP_GameInstance_C|GetSelectedDifficultyLevelhggf _asbp_game_instance) "NewEnumerator2")
              (Variables|Default|SetRemainingTime (.HardInitialTime (Utilities|Struct|BreakS_TrackData _output_get_2)))
              (Variables|Default|SetCheckpointTimeBonus (.HardCheckpointBonus (Utilities|Struct|BreakS_TrackData _output_get_2)))
              (goto _label))))))
    (:then_2
      ;[0.15 0.15 0.15 0.5] Time taken to complete the race calculation
      (if (Utilities|Enum|Equal(Enum) (Variables|Default|GetRaceState) "NewEnumerator1")
        (bind _returnvalue_6 (Utilities|Time|SetTimerbyEvent (delegate Custom|TillRaceComplete) 1.0 true))
        (Variables|Default|SetNewVar _returnvalue_6)
        (else
          (Utilities|Time|ClearandInvalidateTimerbyHandle (Variables|Default|GetNewVar)))))))

(fn ConstructionScript)

(fn OnCheckpointReached
  (params (IncommingIndex :type Integer))
  (if (Utilities|Enum|Equal(Enum) (Variables|Default|GetRaceState) "NewEnumerator1")
    (if (== IncommingIndex (+ (Variables|Default|GetCurrentCheckpointIndex) 1))
      (Math|Integer|IncrementInt (Variables|Default|GetCurrentCheckpointIndex)
        (:%20%20
          (Variables|Default|SetRemainingTime (+ (Variables|Default|GetRemainingTime) (Variables|Default|GetCheckpointTimeBonus)))
          (if (== (Variables|Default|GetCurrentCheckpointIndex) (.TotalCheckpoint (Utilities|Struct|BreakS_TrackData (Variables|Default|GetTrackData))))
            (bind _asbp_player_controller (Utilities|Casting|CastToBP_PlayerController (Game|GetPlayerController 0)))
            (Variables|Default|SetRaceState "NewEnumerator2")
            (Utilities|Time|ClearandInvalidateTimerbyHandle (Variables|Default|GetRaceTimerHandle))
            (CallFunction|GiveRewardsNew)
            (Viewport|RemoveAllWidgets)
            (Default|SwitchtoCinematicCamera _asbp_player_controller)
            (Default|ShowRewardsUIWin _asbp_player_controller (Variables|Default|GetFinalReward) (Variables|Default|GetTotal_Money_After_Win) (Variables|Default|GetTOTAL_TIME%20))))))))

(fn GiveRewardsNew
  (bind _trackdata (Variables|Default|GetTrackData))
  (bind (_name _totalcheckpoint _difficultytier _easyinitialtime _easycheckpointbonus _mediuminitialtime _mediumcheckpointbonus _hardinitialtime _hardcheckpointbonus) (Utilities|Struct|BreakS_TrackData _trackdata))
  (bind _outactors (Actor|GetAllActorsOfClass "/Game/GAMERULES/BP_TrackInfo.BP_TrackInfo_C"))
  (bind _asbp_game_instance (Utilities|Casting|CastToBP_GameInstance (Game|GetGameInstance)))
  (Variables|Default|SetDifficulty%20Tier _difficultytier)
  (switch Utilities|FlowControl|Switch|SwitchonE_Difficulty (Variables|/Game/SHOWROOM/MAIN/BP_GameInstance.BP_GameInstance_C|GetSelectedDifficultyLevelhggf _asbp_game_instance)
    (:NewEnumerator0
      (Variables|Default|SetRemainingTime _easyinitialtime)
      (Variables|Default|SetCheckpointTimeBonus _easycheckpointbonus)
      (Variables|Default|SetFinalReward 25000))
    (:NewEnumerator1
      (Variables|Default|SetRemainingTime _mediuminitialtime)
      (Variables|Default|SetCheckpointTimeBonus _mediumcheckpointbonus)
      (Variables|Default|SetFinalReward 55000))
    (:NewEnumerator2
      (Variables|Default|SetRemainingTime _hardinitialtime)
      (Variables|Default|SetCheckpointTimeBonus _hardcheckpointbonus)
      (Variables|Default|SetFinalReward 110000)))
  (bind _output_get (Variables|Default|SetSaveGameRef (Class|EMSFunctionLibrary|GetCustomSave "/Game/SHOWROOM/MAIN/BP_PlayerCustomSave.BP_PlayerCustomSave_C")))
  (bind _output_get_2 (Variables|/Game/SHOWROOM/MAIN/BP_PlayerCustomSave.BP_PlayerCustomSave_C|SetPlayerCurrency _output_get (+ (Variables|/Game/SHOWROOM/MAIN/BP_PlayerCustomSave.BP_PlayerCustomSave_C|GetPlayerCurrency _output_get) (Variables|Default|GetFinalReward))))
  (switch Utilities|FlowControl|Switch|SwitchonE_Difficulty (Variables|Default|GetSelected%20Difficulty%20Levelhggf)
    (:NewEnumerator0
      (CallFunction|UpdateMapandCheckUnlocks 1 (Utilities|String|StringToName (Variables|Default|GetCurrentMapNamePlayed))))
    (:NewEnumerator1
      (CallFunction|UpdateMapandCheckUnlocks 2 (Utilities|String|StringToName (Variables|Default|GetCurrentMapNamePlayed))))
    (:NewEnumerator2
      (CallFunction|UpdateMapandCheckUnlocks 3 (Utilities|String|StringToName (Variables|Default|GetCurrentMapNamePlayed)))))
  (Class|EMSFunctionLibrary|SaveCustom (Variables|Default|GetSaveGameRef))
  (Variables|Default|SetTotal_Money_After_Win _output_get_2))

(fn UpdateMapandCheckUnlocks
  (params (DiffInt%20 :type Integer) (MapName%20 :type Name))
  (bind _output_get (LocalVariables|SetSave (Class|EMSFunctionLibrary|GetCustomSave "/Game/SHOWROOM/MAIN/BP_PlayerCustomSave.BP_PlayerCustomSave_C")))
  (if (> DiffInt%20 (select (.ReturnValue (Utilities|Map|Find (Variables|/Game/SHOWROOM/MAIN/BP_PlayerCustomSave.BP_PlayerCustomSave_C|GetMapClearRecord _output_get) MapName%20)) (.Value (Utilities|Map|Find (Variables|/Game/SHOWROOM/MAIN/BP_PlayerCustomSave.BP_PlayerCustomSave_C|GetMapClearRecord _output_get) MapName%20)) 0))
    (Utilities|Map|Add (Variables|/Game/SHOWROOM/MAIN/BP_PlayerCustomSave.BP_PlayerCustomSave_C|GetMapClearRecord (LocalVariables|GetSave)) MapName%20 DiffInt%20))
  (LocalVariables|SetMoney (Variables|/Game/SHOWROOM/MAIN/BP_PlayerCustomSave.BP_PlayerCustomSave_C|GetPlayerCurrency (LocalVariables|GetSave)))
  (LocalVariables|SetDesertBest (select (.ReturnValue (Utilities|Map|Find (Variables|/Game/SHOWROOM/MAIN/BP_PlayerCustomSave.BP_PlayerCustomSave_C|GetMapClearRecord (LocalVariables|GetSave)) "Desert")) (.Value (Utilities|Map|Find (Variables|/Game/SHOWROOM/MAIN/BP_PlayerCustomSave.BP_PlayerCustomSave_C|GetMapClearRecord (LocalVariables|GetSave)) "Desert")) 0))
  (LocalVariables|SetKashmirBest (select (.ReturnValue (Utilities|Map|Find (Variables|/Game/SHOWROOM/MAIN/BP_PlayerCustomSave.BP_PlayerCustomSave_C|GetMapClearRecord (LocalVariables|GetSave)) "Kashmir")) (.Value (Utilities|Map|Find (Variables|/Game/SHOWROOM/MAIN/BP_PlayerCustomSave.BP_PlayerCustomSave_C|GetMapClearRecord (LocalVariables|GetSave)) "Kashmir")) 0))
  (LocalVariables|SetGarden_of_Despair1_BEST (select (.ReturnValue (Utilities|Map|Find (Variables|/Game/SHOWROOM/MAIN/BP_PlayerCustomSave.BP_PlayerCustomSave_C|GetMapClearRecord (LocalVariables|GetSave)) "Garden_of_Despair1")) (.Value (Utilities|Map|Find (Variables|/Game/SHOWROOM/MAIN/BP_PlayerCustomSave.BP_PlayerCustomSave_C|GetMapClearRecord (LocalVariables|GetSave)) "Garden_of_Despair1")) 0))
  (bind _output_get_2 (LocalVariables|SetSakuraBest (select (.ReturnValue (Utilities|Map|Find (Variables|/Game/SHOWROOM/MAIN/BP_PlayerCustomSave.BP_PlayerCustomSave_C|GetMapClearRecord (LocalVariables|GetSave)) "Sakura")) (.Value (Utilities|Map|Find (Variables|/Game/SHOWROOM/MAIN/BP_PlayerCustomSave.BP_PlayerCustomSave_C|GetMapClearRecord (LocalVariables|GetSave)) "Sakura")) 0)))
  (if (and (>= _output_get_2 1) (>= (LocalVariables|GetMoney) 120000))
    (Variables|/Game/SHOWROOM/MAIN/BP_PlayerCustomSave.BP_PlayerCustomSave_C|SetbCar2Unlocked (LocalVariables|GetSave) true))
  (if (and (>= (LocalVariables|GetMoney) 280000) (>= _output_get_2 2))
    (Variables|/Game/SHOWROOM/MAIN/BP_PlayerCustomSave.BP_PlayerCustomSave_C|SetbCar3Unlocked (LocalVariables|GetSave) true))
  (if (and (>= (LocalVariables|GetMoney) 550000) (>= (LocalVariables|GetDesertBest) 2))
    (Variables|/Game/SHOWROOM/MAIN/BP_PlayerCustomSave.BP_PlayerCustomSave_C|SetbCar4Unlocked (LocalVariables|GetSave) true))
  (if (and (>= (LocalVariables|GetMoney) 900000) (>= (LocalVariables|GetKashmirBest) 1))
    (Variables|/Game/SHOWROOM/MAIN/BP_PlayerCustomSave.BP_PlayerCustomSave_C|SetbCar5Unlocked (LocalVariables|GetSave) true))
  (if (and (>= (LocalVariables|GetMoney) 1400000) (>= (LocalVariables|GetKashmirBest) 2))
    (Variables|/Game/SHOWROOM/MAIN/BP_PlayerCustomSave.BP_PlayerCustomSave_C|SetbCar6Unlocked (LocalVariables|GetSave) true))
  (if (and (>= (LocalVariables|GetMoney) 2100000) (>= (LocalVariables|GetGarden_of_Despair1_BEST) 2))
    (Variables|/Game/SHOWROOM/MAIN/BP_PlayerCustomSave.BP_PlayerCustomSave_C|SetbCar7Unlocked (LocalVariables|GetSave) true))
  (Class|EMSFunctionLibrary|SaveCustom (LocalVariables|GetSave)))