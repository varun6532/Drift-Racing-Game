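; Garage camera actor that steps through the player's owned vehicles, copying the selected index to the game instance every tick.
; Next/previous events change the index, then set a target X from car spacing and play a timeline intended to lerp the camera there.
; BP_MAINSHOWROOM widgets show only for the matching index.
; Wrapping from last to first resets the index without moving the camera or updating widgets.
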(event Custom|MoveToNextCar
  (if (>= (+ (Variables|Default|GetCurrentCarIndex%20) 1) (Variables|Default|GetMaxCars%20))
    (bind _output_get (Variables|Default|SetCurrentCarIndex%20 0))
    (Default|CallOnCheckpointIndexChanged _output_get)
    (Development|PrintString (Utilities|String|ToString(Integer) _output_get))
    (else
      (bind _result (Math|Integer|IncrementInt (Variables|Default|GetCurrentCarIndex%20))
        (:%20%20
          (Default|CallOnCheckpointIndexChanged _result)
          (Development|PrintString (Utilities|String|ToString(Integer) _result))
          (bind _output_get_2 (Variables|Default|SetCurrentCarIndex%20 (Math|Integer|Clamp(Integer) (Variables|Default|GetCurrentCarIndex%20) 0 (- (Variables|Default|GetMaxCars%20) 1))))
          (Default|CallOnCheckpointIndexChanged _output_get_2)
          (CallFunction|MoveCameratoIndex _output_get_2 (Variables|Default|GetTL_MoveCamera))
          (CallFunction|UpdateVisibleCar))))))

(event Custom|MoveToPreviousCar
  (if (< (- (Variables|Default|GetCurrentCarIndex%20) 1) 0)
    (if (== (Variables|Default|GetCurrentCarIndex%20) 0)
      (bind _output_get (Variables|Default|SetCurrentCarIndex%20 0))
      (Default|CallOnCheckpointIndexChanged _output_get)
      (Development|PrintString (Utilities|String|ToString(Integer) _output_get))
      (Development|PrintString "VARUN"))
    (else
      (bind _result (Math|Integer|DecrementInt (Variables|Default|GetCurrentCarIndex%20))
        (:%20%20
          (Default|CallOnCheckpointIndexChanged _result)
          (Development|PrintString (Utilities|String|ToString(Integer) _result))
          (bind _output_get_2 (Variables|Default|SetCurrentCarIndex%20 (Math|Integer|Clamp(Integer) (Variables|Default|GetCurrentCarIndex%20) 0 (- (Variables|Default|GetMaxCars%20) 1))))
          (Default|CallOnCheckpointIndexChanged _output_get_2)
          (Development|PrintString "Hello")
          (CallFunction|MoveCameratoIndex _output_get_2 (Variables|Default|GetTL_MoveCamera))
          (CallFunction|UpdateVisibleCar))))))

(event EventTick
  (params (DeltaSeconds :type Float%20%28single-precision%29))
  (bind _asbp_game_instance (Utilities|Casting|CastToBP_GameInstance (Game|GetGameInstance)))
  (Variables|/Game/SHOWROOM/MAIN/BP_GameInstance.BP_GameInstance_C|SetCarIndex _asbp_game_instance (Variables|Default|GetCurrentCarIndex%20)))

(event Collision|EventActorBeginOverlap
  (params (OtherActor :type Actor%20Object%20Reference)))

(event EventBeginPlay
  (Transformation|SetWorldLocation (Variables|Default|GetCamera) (Math|Vector|Lerp(Vector) (Variables|Default|GetStartLocation) (Variables|Default|GetTargetLocation%20) (stale _alpha)) false false)
  (Development|PrintString "ekfgeyugfeaygfieydfgedf")
  (Variables|Default|SetMaxCars%20 (Utilities|Array|Length (Variables|/Game/SHOWROOM/MAIN/BP_PlayerCustomSave.BP_PlayerCustomSave_C|GetOwnedVehicles (Class|EMSFunctionLibrary|GetCustomSave "/Game/SHOWROOM/MAIN/BP_PlayerCustomSave.BP_PlayerCustomSave_C"))))
  (CallFunction|UpdateVisibleCar))

(fn ConstructionScript)

(fn CameraMovementCaluator
  (bind _output_get (Variables|Default|SetTargetLocation%20 (Math|Vector|MakeVector (+ (* (Variables|Default|GetCurrentCarIndex%20) (Variables|Default|GetCarSpacing%20)) (.x (Variables|Default|GetTargetLocation%20))) (.y (Variables|Default|GetTargetLocation%20)) (.z (Variables|Default|GetTargetLocation%20)))))
  (Development|PrintString (Utilities|String|ToString(Vector) _output_get))
  (Transformation|SetWorldLocation (Variables|Default|GetCamera) (Math|Interpolation|VInterpTo (Transformation|GetWorldLocation (Variables|Default|GetCamera)) (Variables|Default|GetTargetLocation%20) (Variables|Default|GetDelta%20Seconds) (Variables|Default|GetInterpSpeed%20)) false false))

(fn MoveCameratoIndex
  (params (NewIndex :type Integer) (timreline :type Timeline%20Component%20Object%20Reference))
  (Variables|Default|SetStartLocation (Transformation|GetWorldLocation (Variables|Default|GetCamera)))
  (bind _output_get (Variables|Default|SetTargetLocation%20 (Math|Vector|MakeVector (+ (* NewIndex (Variables|Default|GetCarSpacing%20)) (Variables|Default|GetNewVar)) -4.01e+03 1.4e+02)))
  (Development|PrintString (Utilities|String|ToString(Vector) _output_get) true true "(R=1.000000,G=0.000000,B=0.015327,A=1.000000)" 99999.0)
  (Components|Timeline|PlayfromStart timreline))

(fn UpdateVisibleCar
  (bind _outactors (Actor|GetAllActorsOfClass "/Game/SHOWROOM/MAIN/SHOWROOM/BP_MAINSHOWROOM.BP_MAINSHOWROOM_C"))
  (for _array_element _outactors
    (if (== (Variables|/Game/SHOWROOM/MAIN/SHOWROOM/BP_MAINSHOWROOM.BP_MAINSHOWROOM_C|GetCarIndexShowroomUISetter _array_element) (Variables|Default|GetCurrentCarIndex%20))
      (Default|SetWidgetVisibility _array_element true)
      (else
        (Default|SetWidgetVisibility _array_element false)))))