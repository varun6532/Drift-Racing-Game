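; Showroom car actor that displays a vehicle's name, price and stats and handles buying it, also serving the Garage level.
; BeginPlay creates a WB_CarInfoCard and binds to the level camera's checkpoint-index event.
; Tick refreshes that card by level, using the camera index for the garage and CarIndexShowroomUISetter for the showroom.
; Purchases check saved currency and ownership, then call the GameInstance's AddOwnedVehicle or show a no-money widget.
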(event Custom|OnCheckpointIndex_Received
  (params (NewIndex :type Integer))
  (Variables|Default|SetIndex NewIndex))

(event Custom|SetWidgetVisibility
  (params (IsVisible? :type Boolean))
  (if (not IsVisible?)
    (Class|WidgetComponent|SetTintColorandOpacity (Variables|Default|GetWidget) "(R=0.000000,G=0.000000,B=0.000000,A=0.200000)")))

(event EventBeginPlay
  (bind _returnvalue (UserInterface|CreateWidget "/Game/Garage_ALL/GarageSystem/WB_CarInfoCard.WB_CarInfoCard_C" (Game|GetPlayerController 0)))
  (UserInterface|SetWidget (Variables|Default|GetWidget) _returnvalue)
  (bind _returnvalue_2 (Game|GetCurrentLevelName true))
  (if (Utilities|Enum|Equal(Enum) _returnvalue_2 "Garage_Level")
    (bind _outactors (Actor|GetAllActorsOfClass "/Game/Garage_ALL/GarageSystem/BP_GarageCamera.BP_GarageCamera_C"))
    (bind _output_get (Variables|Default|SetCamRefGarage _outactors))
    (EventDispatchers|BindEventtoOnCheckpointIndexChanged _output_get (delegate Custom|OnCheckpointIndex_Received))
    (else
      (bind _outactors_2 (Actor|GetAllActorsOfClass "/Game/SHOWROOM/MAIN/BP_ShowRoomCamera.BP_ShowRoomCamera_C"))
      (bind _output_get_2 (Variables|Default|SetCamRefShowroom (Utilities|Array|Get(acopy) _outactors_2)))
      (EventDispatchers|BindEventtoOnCheckpointIndexChanged _output_get_2 (delegate Custom|OnCheckpointIndex_Received)))))

(event Collision|EventActorBeginOverlap
  (params (OtherActor :type Actor%20Object%20Reference)))

(event EventTick
  (params (DeltaSeconds :type Float%20%28single-precision%29))
  (CallFunction|AddWidgetsComponetCar))

(fn ConstructionScript)

(fn SHOWATTRIBUTES
  (Utilities|FlowControl|Sequence
    (:then_0
      (Rendering|Components|TextRender|SetText (Variables|Default|GetPrice_text) (Utilities|Text|ToText(Integer) (Variables|Default|GetPrice_of_Car_Int))))
    (:then_1
      (Rendering|Components|TextRender|SetText (Variables|Default|GetNAME%20OF%20CAR) (Utilities|Text|ToText(Name) (Variables|Default|GetName)))))
  (Rendering|SetVisibility (Variables|Default|GetAcceleration) true false))

(fn HIDEATTRIBUTES
  (Rendering|SetVisibility (Variables|Default|GetAcceleration) false false))

(fn BuyingVehicle
  (params (NameOfVEHILETOBUY :type Name))
  (bind _price_of_car_int (Variables|Default|GetPrice_of_Car_Int))
  (Utilities|FlowControl|Sequence
    (:then_0
      (bind _returnvalue (CallFunction|HasOwnedbyName NameOfVEHILETOBUY))
      (if _returnvalue
        (Variables|Default|SetOwned true)
        (else
          (Variables|Default|SetOwned false))))
    (:then_1
      (if (>= (Variables|/Game/SHOWROOM/MAIN/BP_PlayerCustomSave.BP_PlayerCustomSave_C|GetPlayerCurrency (Class|EMSFunctionLibrary|GetCustomSave "/Game/SHOWROOM/MAIN/BP_PlayerCustomSave.BP_PlayerCustomSave_C")) _price_of_car_int)
        (if (Variables|Default|GetOwned)
          (Development|PrintString "Already Owned !!!!!!!!!")
          (else
            (bind _asbp_game_instance (Utilities|Casting|CastToBP_GameInstance (Game|GetGameInstance)))
            (Development|PrintString "Calling the addowned fxn")
            (Default|AddOwnedVehicle _asbp_game_instance NameOfVEHILETOBUY (Variables|Default|GetPrice_of_Car_Int) (Variables|Default|GetMODEL_SHOWROOM) (Variables|Default|GetIMAGE%20OF%20CAR%20) (Variables|Default|GetModel) (Variables|Default|GetTopSpeedRating) (Variables|Default|GetAccelerationRating) (Variables|Default|GetHandlingRating) (Variables|Default|GetBrakingRating))
            (Development|PrintString "Called  the addowned fxn")
            (return)))
        (else
          (bind _returnvalue_2 (UserInterface|CreateWidget "/Game/UI/NomoneyUI/WBP_NOMONEY.WBP_NOMONEY_C"))
          (UserInterface|Viewport|AddtoViewport _returnvalue_2 0))))
    (:then_2
      (Development|PrintString (Utilities|String|ToString(Integer) _price_of_car_int)))))

(fn AddOwnedVehicle(STRUCT)
  (params (Car :type CAR%20STRUCT%20Structure))
  (Utilities|Array|AddUnique (Variables|/Game/SHOWROOM/MAIN/BP_PlayerCustomSave.BP_PlayerCustomSave_C|GetOwnedVehicles (Class|EMSFunctionLibrary|GetCustomSave "/Game/SHOWROOM/MAIN/BP_PlayerCustomSave.BP_PlayerCustomSave_C")) Car)
  (Class|EMSFunctionLibrary|SaveCustom)
  (Development|PrintString "aDDED THE CAR FOR STRUCT"))

(fn HasOwnedbyName
  (params (Name :type Name))
  (for _array_element (Variables|/Game/SHOWROOM/MAIN/BP_PlayerCustomSave.BP_PlayerCustomSave_C|GetOwnedVehicles (Class|EMSFunctionLibrary|GetCustomSave "/Game/SHOWROOM/MAIN/BP_PlayerCustomSave.BP_PlayerCustomSave_C"))
    (return (Utilities|Enum|Equal(Enum) (Utilities|String|ToString(Text) (.Name (Utilities|Struct|BreakCAR_STRUCT _array_element))) (Utilities|String|ToString(Name) Name)))))

(fn ShowVehicles
  (for _array_element (Variables|/Game/SHOWROOM/MAIN/BP_PlayerCustomSave.BP_PlayerCustomSave_C|GetOwnedVehicles (Class|EMSFunctionLibrary|GetCustomSave "/Game/SHOWROOM/MAIN/BP_PlayerCustomSave.BP_PlayerCustomSave_C"))
    (Development|PrintText (.name _array_element))))

(fn AddWidgetsComponetCar
  (bind _aswb_car_info_card (Utilities|Casting|CastToWB_CarInfoCard (UserInterface|GetWidget (Variables|Default|GetWidget))))
  (bind _returnvalue (Game|GetCurrentLevelName true))
  (if (Utilities|Enum|Equal(Enum) _returnvalue "Showroom_Level")
    (Default|UpdateDisplayShowroom _aswb_car_info_card (Variables|Default|GetCarIndexShowroomUISetter))
    (else
      (Default|UpdatedISPALYGarage _aswb_car_info_card (Variables|Default|GetIndex)))))

(fn ComponentstoSave
  (return 0))