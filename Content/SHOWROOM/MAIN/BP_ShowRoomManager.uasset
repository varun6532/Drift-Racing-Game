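; BP_ShowRoomManager fills the showroom with the player's owned vehicles when play begins.
; It reads the OwnedVehicles list from BP_PlayerCustomSave, then finds every BP_CarSpawnPoint in the level.
; Each point's SpawnIndex selects a vehicle entry, whose Model class is spawned at that point's transform and stored in SpawedActors.
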(event EventBeginPlay
  (Variables|Default|SetOwned%20Vehicle (Variables|/Game/SHOWROOM/MAIN/BP_PlayerCustomSave.BP_PlayerCustomSave_C|GetOwnedVehicles (Class|EMSFunctionLibrary|GetCustomSave "/Game/SHOWROOM/MAIN/BP_PlayerCustomSave.BP_PlayerCustomSave_C")))
  (bind _outactors (Actor|GetAllActorsOfClass "/Game/Garage_ALL/GarageSystem/BP_CarSpawnPoint.BP_CarSpawnPoint_C"))
  (for _array_element _outactors
    (Utilities|IsValid self
      (:Is%20Valid
        (bind _returnvalue (Game|SpawnActorfromClass (.Model (Utilities|Struct|BreakCAR_STRUCT (Utilities|Array|Get(acopy) (Variables|Default|GetOwned%20Vehicle) (Variables|/Game/Garage_ALL/GarageSystem/BP_CarSpawnPoint.BP_CarSpawnPoint_C|GetSpawnIndex%20 _array_element)))) (Transformation|GetActorTransform _array_element) "Undefined" "MultiplyWithRoot" 0 0))
        (bind _returnvalue_2 (Utilities|Array|Add (Variables|Default|GetSpawedActors) _returnvalue))))))

(event Collision|EventActorBeginOverlap
  (params (OtherActor :type Actor%20Object%20Reference)))

(event EventTick
  (params (DeltaSeconds :type Float%20%28single-precision%29)))

(fn ConstructionScript)