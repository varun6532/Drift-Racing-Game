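; Showroom display Blueprint for the Kerosene car, showing its model and stats.
; On BeginPlay it runs two setup functions, both reading a hardcoded entry in the CARSALLSHOWROOM car list.
; Attributes fills text components with name, acceleration, steering and top speed in km/h.
; BodyAndWheel assigns the body mesh and applies one shared wheel mesh to all four wheels.
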(event EventBeginPlay
  (|CallParentFunction)
  (Utilities|FlowControl|Sequence
    (:then_0
      (CallFunction|Attributes))
    (:then_1
      (CallFunction|BodyandWheel))))

(event Collision|EventActorBeginOverlap
  (params (OtherActor :type Actor%20Object%20Reference))
  (|CallParentFunction OtherActor) ; This node is disabled and will not be called.\nDrag off pins to build functionality.
)

(event EventTick
  (params (DeltaSeconds :type Float%20%28single-precision%29))
  (|CallParentFunction DeltaSeconds) ; This node is disabled and will not be called.\nDrag off pins to build functionality.
)

(fn ConstructionScript
  (|CallParentFunction))

(fn Attributes
  (bind _cars_all_showroom (Variables|Default|GetCARS_ALL_SHOWROOM))
  (bind _output (Utilities|Array|Get(acopy) _cars_all_showroom))
  (bind _carslist (Utilities|Struct|BreakBP_CARLIST_SHOWROOM _output))
  (bind _output_2 (Utilities|Array|Get(acopy) _carslist 8))
  (bind (_name _isai_ _bodymesh _wheelmesh _wheelmeshoffset _springdamping _springcoeficient _idlesound _revsound _acceleration _breakingpower _steering _snapsteering _traction _maxspeedinkmh) (Utilities|Struct|BreakBP_CarSpecs _output_2))
  (Utilities|FlowControl|Sequence
    (:then_0
      ;[0.15 0.15 0.15 0.5] attributes setter
      (Rendering|Components|TextRender|SetText (Variables|Default|GetNAME%20OF%20CAR) (Utilities|Text|ToText(String) _name)))
    (:then_1
      (Rendering|Components|TextRender|SetText (Variables|Default|GetAcceleration%20Value) (Utilities|Text|ToText(Float) _acceleration "HalfToEven")))
    (:then_2
      (Rendering|Components|TextRender|SetText (Variables|Default|GetSteering%20VALUE) (Utilities|Text|ToText(Float) _steering "HalfToEven")))
    (:then_3
      (Rendering|Components|TextRender|SetText (Variables|Default|GetMaximum%20Speed%20Value) (Utilities|Text|ToText(Float) _maxspeedinkmh "HalfToEven")))))

(fn BodyandWheel
  (bind _cars_all_showroom (Variables|Default|GetCARS_ALL_SHOWROOM))
  (bind _output (Utilities|Array|Get(acopy) _cars_all_showroom))
  (bind _carslist (Utilities|Struct|BreakBP_CARLIST_SHOWROOM _output))
  (bind _output_2 (Utilities|Array|Get(acopy) _carslist 8))
  (bind (_name _isai_ _bodymesh _wheelmesh) (Utilities|Struct|BreakBP_CarSpecs _output_2))
  (Utilities|FlowControl|Sequence
    (:then_0
      ;[0.15 0.15 0.15 0.5] BODY AND WHEEL SETUP
      (Components|StaticMesh|SetStaticMesh (Variables|Default|GetBody_0) _bodymesh))
    (:then_1
      (Components|StaticMesh|SetStaticMesh (Variables|Default|GetWheel_RR) _wheelmesh))
    (:then_2
      (Components|StaticMesh|SetStaticMesh (Variables|Default|GetWheel_RL) _wheelmesh))
    (:then_3
      (Components|StaticMesh|SetStaticMesh (Variables|Default|GetWheel_FL) _wheelmesh))
    (:then_4
      (Components|StaticMesh|SetStaticMesh (Variables|Default|GetWheel_FR) _wheelmesh))))