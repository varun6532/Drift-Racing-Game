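; BP_AI_BrakeVolume is a trigger volume that slows AI drift cars to a desired speed in km/h.
; Overlap events track AI-controlled BP_MainDirftController cars entering and leaving the volume.
; Each Tick, cars above the target horizontal speed get a braking flag and have their physics velocity directly scaled down by their BreakingPower.
; Cars at or below that speed, or leaving the volume, are released and untracked.
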(event OnComponentBeginOverlap(BrakeVolumeCol)
  (params (OverlappedComponent :type Primitive%20Component%20Object%20Reference) (OtherActor :type Actor%20Object%20Reference) (OtherComp :type Primitive%20Component%20Object%20Reference) (OtherBodyIndex :type Integer) (bFromSweep :type Boolean) (SweepResult :type Hit%20Result%20Structure%20%28by%20ref%29))
  (bind _asbp_main_dirft_controller (Utilities|Casting|CastToBP_MainDirftController OtherActor))
  (if (Variables|/Game/DriftMaster/Blueprints/BP_MainDirftController.BP_MainDirftController_C|GetIs%20AI? _asbp_main_dirft_controller)
    (Utilities|Array|Add (Variables|Default|GetCarsInside) _asbp_main_dirft_controller)))

(event OnComponentEndOverlap(BrakeVolumeCol)
  (params (OverlappedComponent :type Primitive%20Component%20Object%20Reference) (OtherActor :type Actor%20Object%20Reference) (OtherComp :type Primitive%20Component%20Object%20Reference) (OtherBodyIndex :type Integer))
  (bind _asbp_main_dirft_controller (Utilities|Casting|CastToBP_MainDirftController OtherActor))
  (if (Utilities|Array|ContainsItem (Variables|Default|GetCarsInside) _asbp_main_dirft_controller)
    (Utilities|Array|RemoveItem (Variables|Default|GetCarsInside) _asbp_main_dirft_controller)
    (Variables|/Game/DriftMaster/Blueprints/BP_MainDirftController.BP_MainDirftController_C|SetAI%20Is%20Braking _asbp_main_dirft_controller false)))

(event EventTick
  (params (DeltaSeconds :type Float%20%28single-precision%29))
  (bind _carsinside (Variables|Default|GetCarsInside))
  (if (Utilities|Array|IsNotEmpty _carsinside)
    (for _array_element _carsinside
      (if (> (Math|Vector|VectorLengthXY (Transformation|GetComponentVelocity (Variables|/Game/DriftMaster/Blueprints/BP_MainDirftController.BP_MainDirftController_C|GetMainBody _array_element))) (/ (Variables|Default|GetDesired%20Speed%20in%20KM/H) 0.036))
        (Variables|/Game/DriftMaster/Blueprints/BP_MainDirftController.BP_MainDirftController_C|SetAI%20Is%20Braking _array_element true)
        (Physics|SetPhysicsLinearVelocity (Variables|/Game/DriftMaster/Blueprints/BP_MainDirftController.BP_MainDirftController_C|GetMainBody _array_element) (* (Transformation|GetComponentVelocity (Variables|/Game/DriftMaster/Blueprints/BP_MainDirftController.BP_MainDirftController_C|GetMainBody _array_element)) (- 1.0 (Variables|/Game/DriftMaster/Blueprints/BP_MainDirftController.BP_MainDirftController_C|GetBreakingPower _array_element))) false "None")
        (elif (Utilities|Array|ContainsItem (Variables|Default|GetCarsInside) _array_element)
          (Variables|/Game/DriftMaster/Blueprints/BP_MainDirftController.BP_MainDirftController_C|SetAI%20Is%20Braking _array_element false)
          (Utilities|Array|RemoveItem (Variables|Default|GetCarsInside) _array_element))))))

(fn ConstructionScript)