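; Per-wheel raycast suspension component for the drift car owned by BP_MainDirftController.
; Each tick it traces downward and, on ground contact, applies a vertical spring-damper force to the car's root at its location.
; It places the child wheel and emitter from the trace, spinning the wheel by car velocity except when handbraking with RWD set.
; The spring and wheel-offset setter events are empty, their assignments unwired.
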(event Custom|Set%20Spring%20Values
  (params (SpringCoeficient :type Float%20%28double-precision%29) (DampingCoeficient :type Float%20%28double-precision%29)))

(event Custom|Set%20Wheel%20Offset
  (params (WheelMeshOffset :type Float%20%28double-precision%29)))

(event EventBeginPlay
  (bind _asbp_main_dirft_controller (Utilities|Casting|CastToBP_MainDirftController (Components|GetOwner)))
  (Variables|Default|SetPlayerRef _asbp_main_dirft_controller)
  (Variables|Default|SetWheelRef (Components|GetChildComponent 0))
  (Variables|Default|SetContinueWork true))

(event EventTick
  (params (DeltaSeconds :type Float%20%28single-precision%29))
  (bind _returnvalue (Transformation|GetWorldLocation))
  (bind _returnvalue_2 (Transformation|GetWorldLocation))
  (bind _playerref (Variables|Default|GetPlayerRef))
  (bind _wheelref (Variables|Default|GetWheelRef))
  (bind _emmiterref (Variables|Default|GetEmmiterRef))
  (if (Variables|Default|GetContinueWork)
    (bind (_outhit _returnvalue_3) (Collision|LineTraceByChannel (Math|Vector|MakeVector (.x _returnvalue) (.y _returnvalue) (+ (.z _returnvalue) 5e+01)) (+ (Transformation|GetWorldLocation) (* (Math|Vector|GetUpVector) (* (Math|Float|MakeLiteralFloat 5e+01) -1.0))) "TraceTypeQuery1" false 0 "None"))
    (Utilities|FlowControl|Sequence
      (:then_0
        (bind _output_get (Variables|Default|SetOnGround _returnvalue_3))
        (if _output_get
          (bind _output_get_2 (Variables|Default|SetPosDelta (- 1e+02 (.Distance (Collision|BreakHitResult _outhit)))))
          (Class|PrimitiveComponent|AddForceatLocation (.AsPrimitive%20Component (Utilities|Casting|CastToPrimitiveComponent (Variables|/Script/Engine.Actor|GetRootComponent (Variables|Default|GetPlayerRef)))) (Math|Vector|MakeVector 0.0 0.0 (+ (* (/ (- _output_get_2 (Variables|Default|GetPrevPosDelta)) (Utilities|Time|GetWorldDeltaSeconds)) (Variables|Default|GetDampingCoeficient)) (* _output_get_2 (Variables|Default|GetSpringCoeficient)))) (Transformation|GetWorldLocation) "None")
          (Variables|Default|SetPrevPosDelta (Variables|Default|GetPosDelta))))
      (:then_1
        (Variables|Default|SetImpact%20Normal (.ImpactNormal (Collision|BreakHitResult _outhit)))
        (Utilities|IsValid _wheelref
          (:Is%20Valid
            (Transformation|SetWorldLocation _wheelref (Math|Vector|MakeVector (.x _returnvalue_2) (.y _returnvalue_2) (.z (+ (|WhichPoint (.TraceEnd (Collision|BreakHitResult _outhit)) (.Location (Collision|BreakHitResult _outhit))) (Math|Vector|MakeVector 0.0 0.0 (Variables|Default|GetWheelMeshOffset))))) false false)
            (Utilities|IsValid _emmiterref
              (:Is%20Valid
                (Transformation|SetWorldLocation _emmiterref (+ (|WhichPoint (.TraceEnd (Collision|BreakHitResult _outhit)) (.Location (Collision|BreakHitResult _outhit))) "0.000000,0.000000,1.000000") false true))
              (:Is%20Not%20Valid
                _))
            (if (Variables|/Game/DriftMaster/Blueprints/BP_MainDirftController.BP_MainDirftController_C|GetHandBrake (Variables|Default|GetPlayerRef))
              (if (not (Variables|Default|GetRWD))
                (Transformation|AddLocalRotation (Variables|Default|GetWheelRef) (Math|Rotator|MakeRotator 0.0 (* (* (Math|Vector|VectorLengthXY (Transformation|GetVelocity (Variables|Default|GetPlayerRef))) -0.03) (Math|Vector|DotProduct (Transformation|GetActorForwardVector _playerref) (Math|Vector|Normalize (Transformation|GetVelocity _playerref)))) 0.0) false false :!label _label))
              (else
                (goto _label)))))))))